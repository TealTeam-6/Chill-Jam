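; Game mode that handles level loading and per-level timing.
; It opens levels by index from the game instance's level list, storing the current number and printing the level name.
; A gate on Tick accumulates the timer from BeginPlay, when StartLevel resets it.
; EndLevel shows the level-complete widget, adds the time to the game instance's running total and closes the gate.
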(event Custom|Open%20Level%20%28by%20Number%29
  (params (Level%20Number :type Integer))
  (bind _chill_instance (CallFunction|GetChillGameInstance))
  (bind _chill_levels (Variables|/Game/Blueprints/GameInstance/BPI_ChillGameInstance.BPI_ChillGameInstance_C|GetChill%20Levels _chill_instance))
  (bind _output (Utilities|Array|Get(acopy) _chill_levels Level%20Number))
  (Variables|/Game/Blueprints/GameInstance/BPI_ChillGameInstance.BPI_ChillGameInstance_C|SetCurrent%20Level _chill_instance Level%20Number)
  (Game|OpenLevel(byName) _output)
  (Development|PrintText (Utilities|Text|ToText(Name) _output)))

(event Custom|End%20Level
  (bind _chill_instance (CallFunction|GetChillGameInstance))
  (bind _returnvalue (Game|ConstructObjectfromClass "/Game/Blueprints/Widgets/WBP_LevelComplete.WBP_LevelComplete_C"))
  (UserInterface|Viewport|AddtoViewport _returnvalue 0)
  (Variables|/Game/Blueprints/GameInstance/BPI_ChillGameInstance.BPI_ChillGameInstance_C|SetTotal%20Time _chill_instance (+ (Variables|Default|GetTimer) (Variables|/Game/Blueprints/GameInstance/BPI_ChillGameInstance.BPI_ChillGameInstance_C|GetTotal%20Time _chill_instance)))
  (Utilities|FlowControl|Gate true) ; enters at Close
)

(event Custom|Start%20Level
  (Variables|Default|SetTimer 0.0)
  (CallFunction|StartTimer))

(event Custom|Start%20Timer
  (Utilities|FlowControl|Gate true) ; enters at Open
)

(event EventTick
  (params (DeltaSeconds :type Float%20%28single-precision%29))
  (Utilities|FlowControl|Gate true
    (:Exit
      (Variables|Default|SetTimer (+ (Utilities|Time|GetWorldDeltaSeconds) (Variables|Default|GetTimer))))))

(event EventBeginPlay
  (CallFunction|StartLevel))

(fn ConstructionScript)