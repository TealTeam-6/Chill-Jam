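; BFL_ChillShortcuts is a Blueprint function library of shortcut getters for the Chill game's core framework objects.
; It returns the game mode, game instance, player controller and player character, each already cast to its Chill Blueprint class.
; The controller and character getters always use player index 0, so they only resolve the first player.
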(fn GetChillGamemode
  (return (.AsBP%20Chill%20Gamemode (Utilities|Casting|CastToBP_ChillGamemode (Game|GetGameMode)))))

(fn GetChillGameInstance
  (return (.AsBPI%20Chill%20Game%20Instance (Utilities|Casting|CastToBPI_ChillGameInstance (Game|GetGameInstance)))))

(fn GetChillController
  (return (.AsBP%20Chill%20Controller (Utilities|Casting|CastToBP_ChillController (Game|GetPlayerController 0)))))

(fn GetChillCharacter
  (return (.AsBP%20Chill%20Character (Utilities|Casting|CastToBP_ChillCharacter (Game|Player|GetPlayerPawn 0)))))