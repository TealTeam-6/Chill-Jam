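; Campfire actor that serves as the level's end goal when the player's chill character reaches it.
; Overlapping its box disables player input, zeroes the character's velocity, plays the campfire music and toggles the game instance's music.
; After a five-second delay it tells the game mode to end the level.
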(event OnComponentBeginOverlap(Box)
  (params (OverlappedComponent :type Primitive%20Component%20Object%20Reference) (OtherActor :type Actor%20Object%20Reference) (OtherComp :type Primitive%20Component%20Object%20Reference) (OtherBodyIndex :type Integer) (bFromSweep :type Boolean) (SweepResult :type Hit%20Result%20Structure%20%28by%20ref%29))
  (bind _asbp_chill_character (Utilities|Casting|CastToBP_ChillCharacter OtherActor))
  (Input|DisableInput _asbp_chill_character (Game|GetPlayerController 0))
  (Audio|PlaySound2D "/Game/Sound/W_CampfireMusic.W_CampfireMusic" 1.0 1.0 0.0 0 0)
  (Default|ToogleMusic (CallFunction|GetChillGameInstance))
  (Variables|/Script/Engine.MovementComponent|SetVelocity (Variables|/Script/Engine.Character|GetCharacterMovement (.AsBP%20Chill%20Character (Utilities|Casting|CastToBP_ChillCharacter (Game|GetPlayerCharacter 0)))) "0, 0, 0")
  (Utilities|FlowControl|Delay 5.0)
  (Default|EndLevel (CallFunction|GetChillGamemode)))

(fn ConstructionScript)