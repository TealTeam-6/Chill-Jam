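; ChillSphere is an actor that springs toward the cursor's hit point on Destructible objects, trailing a tube of spline meshes.
; Construction flattens its Y position to zero and creates a pool of Resolution spline mesh segments.
; Tick moves the actor and stretches the current segment's end to it, setting tangent from velocity and scale from a growing Radius.
; A looping delay recycles segments as a ring buffer, chaining each to the previous end.
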(event EventTick
  (params (DeltaSeconds :type Float%20%28single-precision%29))
  (bind _returnvalue (Transformation|GetActorLocation))
  (bind _overlapmeshes (Variables|Default|GetOverlapMeshes))
  (bind _selectedspline (Variables|Default|GetSelectedSpline))
  (bind _output (Utilities|Array|Get(acopy) _overlapmeshes _selectedspline))
  (Variables|Default|SetRadius (+ (Variables|Default|GetRadius) (* DeltaSeconds (Variables|Default|GetRadiusGrowth))))
  (bind _returnvalue_2 (Class|KismetMathLibrary|VectorSpringInterp _returnvalue (.Location (Collision|BreakHitResult (.HitResult (Class|PlayerController|GetHitResultUnderCursorforObjects (Game|GetPlayerController 0) (Utilities|Array|MakeArray "ObjectTypeQuery6") false)))) (Variables|Default|GetSpring%20State) 1e+02 0.2 DeltaSeconds 1e+01 1.0))
  (Utilities|FlowControl|Sequence
    (:then_0
      (SplineMesh|SetEndPosition _output (Transformation|GetActorLocation) true)
      (SplineMesh|SetEndTangent _output (/ (- _returnvalue_2 _returnvalue) DeltaSeconds) true :!class /Script/Engine.SplineMeshComponent)
      (SplineMesh|SetEndScale _output (Math|Vector2D|MakeVector2D (Variables|Default|GetRadius) (Variables|Default|GetRadius)) true :!class /Script/Engine.SplineMeshComponent))
    (:then_1
      (Transformation|SetActorLocation _returnvalue_2 false false))))

(event EventBeginPlay
  (Utilities|FlowControl|Delay (/ (Variables|Default|GetTail%20Length) (Variables|Default|GetResolution)) :!label _label)
  (Variables|Default|SetSelectedSpline (Math|Integer|%(Integer) (+ (Variables|Default|GetSelectedSpline) 1) (Variables|Default|GetResolution)))
  (SplineMesh|SetStartandEnd (Utilities|Array|Get(acopy) (Variables|Default|GetOverlapMeshes) (Variables|Default|GetSelectedSpline)) (SplineMesh|GetEndPosition (Utilities|Array|Get(acopy) (Variables|Default|GetOverlapMeshes) (- (select (< (Variables|Default|GetSelectedSpline) 1) (Variables|Default|GetResolution) (Variables|Default|GetSelectedSpline)) 1))) (SplineMesh|GetEndTangent (Utilities|Array|Get(acopy) (Variables|Default|GetOverlapMeshes) (- (select (< (Variables|Default|GetSelectedSpline) 1) (Variables|Default|GetResolution) (Variables|Default|GetSelectedSpline)) 1))) (Transformation|GetActorLocation) (SplineMesh|GetEndTangent (Utilities|Array|Get(acopy) (Variables|Default|GetOverlapMeshes) (- (select (< (Variables|Default|GetSelectedSpline) 1) (Variables|Default|GetResolution) (Variables|Default|GetSelectedSpline)) 1))) false :!class /Script/Engine.SplineMeshComponent)
  (SplineMesh|SetStartScale (Utilities|Array|Get(acopy) (Variables|Default|GetOverlapMeshes) (Variables|Default|GetSelectedSpline)) (SplineMesh|GetEndScale (Utilities|Array|Get(acopy) (Variables|Default|GetOverlapMeshes) (- (select (< (Variables|Default|GetSelectedSpline) 1) (Variables|Default|GetResolution) (Variables|Default|GetSelectedSpline)) 1))) true :!class /Script/Engine.SplineMeshComponent)
  (goto _label))

(fn ConstructionScript
  (bind _returnvalue (Transformation|GetActorLocation))
  (Transformation|SetActorLocation (* (Transformation|GetActorLocation) "1.000000,0.000000,1.000000") false false)
  (for _index (range 1 (Variables|Default|GetResolution))
    (bind _returnvalue_2 (AddComponent|AddSplineMeshComponent false))
    (SplineMesh|SetStartandEnd _returnvalue_2 _returnvalue "0, 0, 0" _returnvalue "0, 0, 0" true :!class /Script/Engine.SplineMeshComponent)
    (Utilities|Array|Add (Variables|Default|GetOverlapMeshes) _returnvalue_2)))