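; BP_Background is a tiled Paper2D background actor that repeats a sprite along X to form a wider backdrop.
; Its construction script adds AddOns extra sprite components, each offset by a multiple of the base sprite's bounds width and matched to its world scale.
; The copies always use the fixed BackgroundTileable1_Sprite asset.
; An alternative that spawns whole BP_Background actors sits unconnected in the event graph, and BeginPlay does nothing.
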(event EventBeginPlay)

(fn ConstructionScript
  (bind _add_ons (Variables|Default|GetAdd%20Ons))
  (bind _backgroundtileable1_sprite (Variables|Default|GetBackgroundTileable1_Sprite))
  (if (> _add_ons 0)
    (for _index (range 1 _add_ons)
      (bind _returnvalue (AddComponent|AddPaperSpriteComponent false (Math|Transform|MakeTransform (+ (.location (Transformation|GetRelativeTransform (Variables|Default|GetBackgroundTileable1_Sprite))) (Math|Vector|MakeVector (* (* (.x (.BoxExtent (Collision|GetComponentBounds _backgroundtileable1_sprite))) 2.0) _index) 0.0 0.0)) "0, 0, 0" "1.000000,1.000000,1.000000")))
      (Rendering|Components|Sprite|SetSprite _returnvalue "/Game/Decorations/BackgroundTileable1_Sprite.BackgroundTileable1_Sprite")
      (Transformation|SetWorldScale3D _returnvalue (Transformation|GetWorldScale _backgroundtileable1_sprite)))))