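; BP_BasePlatform is a base platform actor that builds its shape from a spline, flattened onto the XZ plane at Y=0.
; The Construction Script adds one spline mesh per TextureSize of spline length, applies Material and stores it in Meshes.
; Segment ends are sampled at constant velocity.
; Tangents are divided by an estimated per-segment stretch ratio and clamped to TextureSize to limit distortion.
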(fn ConstructionScript
  (bind _spline (Variables|Default|GetSpline))
  (bind _spline_2 (Variables|Default|GetSpline))
  (bind _spline_3 (Variables|Default|GetSpline))
  (bind _texturesize (Variables|Default|GetTextureSize))
  (bind _spline_4 (Variables|Default|GetSpline))
  (bind _texturesize_2 (Variables|Default|GetTextureSize))
  (bind _returnvalue (Spline|GetSplineLength _spline_2))
  (bind _returnvalue_2 (Spline|GetSplineLength _spline_3))
  (bind _returnvalue_3 (Spline|GetNumberOfSplinePoints _spline_4))
  (bind _returnvalue_4 (/ _returnvalue _texturesize))
  (Transformation|SetActorLocation (* (Transformation|GetActorLocation) "1.000000,0.000000,1.000000") false false)
  (for _index (range 0 (- _returnvalue_4 1))
    (bind _returnvalue_5 (AddComponent|AddSplineMeshComponent false))
    (Rendering|Material|SetMaterial _returnvalue_5 0 (Variables|Default|GetMaterial))
    (Utilities|Array|Add (Variables|Default|GetMeshes) _returnvalue_5)
    (SplineMesh|SetStartandEnd _returnvalue_5 (* (Spline|GetLocationatTime _spline (/ (Math|Conversions|ToFloat(Integer) _index) _returnvalue_4) "Local" true) "1.000000,0.000000,1.000000") (Math|Vector|ClampVectorSize (/ (* (Class|SplineComponent|GetTangentatTime _spline (/ (Math|Conversions|ToFloat(Integer) _index) _returnvalue_4) "Local" true) "1.000000,0.000000,1.000000") (Utilities|Operators|Divide (- (* _returnvalue_2 (/ (Math|Conversions|ToFloat(Integer) (+ (/ (* (/ (+ (Math|Conversions|ToFloat(Integer) _index) 1) _returnvalue_4) (* _returnvalue_3 10)) 10) 1)) _returnvalue_3)) (* _returnvalue_2 (/ (Math|Conversions|ToFloat(Integer) (/ (* (/ (Math|Conversions|ToFloat(Integer) _index) _returnvalue_4) (* _returnvalue_3 10)) 10)) _returnvalue_3))) (Variables|Default|GetTextureSize) 1.0)) 0.0 _texturesize_2) (* (Spline|GetLocationatTime _spline (/ (+ (Math|Conversions|ToFloat(Integer) _index) 1) _returnvalue_4) "Local" true) "1.000000,0.000000,1.000000") (Math|Vector|ClampVectorSize (/ (* (Class|SplineComponent|GetTangentatTime _spline (/ (+ (Math|Conversions|ToFloat(Integer) _index) 1) _returnvalue_4) "Local" true) "1.000000,0.000000,1.000000") (Utilities|Operators|Divide (- (* _returnvalue_2 (/ (Math|Conversions|ToFloat(Integer) (+ (/ (* (/ (+ (Math|Conversions|ToFloat(Integer) _index) 1) _returnvalue_4) (* _returnvalue_3 10)) 10) 1)) _returnvalue_3)) (* _returnvalue_2 (/ (Math|Conversions|ToFloat(Integer) (/ (* (/ (Math|Conversions|ToFloat(Integer) _index) _returnvalue_4) (* _returnvalue_3 10)) 10)) _returnvalue_3))) (Variables|Default|GetTextureSize) 1.0)) 0.0 _texturesize_2) true :!class /Script/Engine.SplineMeshComponent)))