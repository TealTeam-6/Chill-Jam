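; BP_BasePlatform is a base platform actor that builds its geometry along an editable spline.
; Its construction script prints the spline length, then adds a spline mesh component for roughly every 200 units of length.
; Each segment takes its endpoints and tangents from constant-velocity time sampling in local space, with tangents scaled down by segment count times spline point count.
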(fn ConstructionScript
  (bind _spline (Variables|Default|GetSpline))
  (bind _spline_2 (Variables|Default|GetSpline))
  (bind _returnvalue (Spline|GetNumberOfSplinePoints _spline_2))
  (bind _returnvalue_2 (Spline|GetSplineLength _spline_2))
  (bind _returnvalue_3 (Math|Conversions|ToFloat(Integer) _returnvalue))
  (bind _returnvalue_4 (/ _returnvalue_2 2e+02))
  (bind _returnvalue_5 (* 1.0 _returnvalue_4))
  (bind _returnvalue_6 (* _returnvalue_5 _returnvalue_3))
  (Development|PrintString (Utilities|String|ToString(Float) _returnvalue_2))
  (for _index (range 0 (- _returnvalue_5 1))
    (bind _returnvalue_7 (AddComponent|AddSplineMeshComponent false))
    (SplineMesh|SetStartandEnd _returnvalue_7 (Spline|GetLocationatTime _spline (/ (Math|Conversions|ToFloat(Integer) _index) _returnvalue_5) "Local" true) (/ (Class|SplineComponent|GetTangentatTime _spline (/ (Math|Conversions|ToFloat(Integer) _index) _returnvalue_5) "Local" true) _returnvalue_6) (Spline|GetLocationatTime _spline (/ (+ (Math|Conversions|ToFloat(Integer) _index) 1) _returnvalue_5) "Local" true) (/ (Class|SplineComponent|GetTangentatTime _spline (/ (+ (Math|Conversions|ToFloat(Integer) _index) 1) _returnvalue_5) "Local" true) _returnvalue_6) true :!class /Script/Engine.SplineMeshComponent)))