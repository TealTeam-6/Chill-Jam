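; Side-scrolling player character locked to the XZ plane that walks, jumps and slides on slideable surfaces.
; Tick checks the floor for slideability, switching to Flying movement, where Move applies slope-projected input and manual gravity using a sphere trace.
; The camera root eases between grid-snapped positions, panning screen by screen.
; Time in chill drains an allowance; running out or falling below KillZ resets the character to spawn.
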(event Custom|Reset
  (Transformation|SetActorLocation (Variables|Hidden|GetSpawnLocation) false false)
  (Variables|Default|SetAlowedTimeInChill (.AlowedTimeInChill (Utilities|GetClassDefaults "BP_ChillCharacter_C")))
  (Default|CallOnReset))

(event EventBeginPlay
  (bind _charactermovement (Variables|Character|GetCharacterMovement))
  (Variables|Hidden|SetSpawnLocation (Transformation|GetActorLocation))
  (Variables|Hidden|SetMax%20Acceleration (Class|CharacterMovementComponent|GetMaxAcceleration _charactermovement))
  (Variables|/Script/Engine.MovementComponent|SetVelocity _charactermovement "0, 0, 0"))

(event EventUnappllyChill
  (bind _output_get (Variables|Hidden|SetInChill false))
  (Default|CallOninChillUpdated _output_get))

(event EventApplyChill
  (bind _output_get (Variables|Hidden|SetInChill true))
  (Default|CallOninChillUpdated _output_get))

(event EventTick
  (params (DeltaSeconds :type Float%20%28single-precision%29))
  (bind _charactermovement (Variables|Character|GetCharacterMovement))
  ;[1 1 1] Camera Panning
  (Transformation|SetWorldLocation (Variables|Default|GetCameraRoot) (Math|Interpolation|VInterpTo (Transformation|GetWorldLocation (Variables|Default|GetCameraRoot)) (Class|KismetMathLibrary|VectorSnappedtoGrid (Transformation|GetActorLocation) 5e+03) DeltaSeconds 1.0) false false)
  (Utilities|FlowControl|Sequence
    (:then_0
      ;[1 1 1] Update Sliding
      (if (or (.bBlockingHit (Collision|BreakHitResult (select (Variables|Hidden|GetSliding) (Variables|Hidden|GetFloor%20Hit) (.HitResult (Utilities|Struct|BreakFindFloorResult (Variables|/Script/Engine.CharacterMovementComponent|GetCurrentFloor (Variables|Character|GetCharacterMovement))))))) (.bInitialOverlap (Collision|BreakHitResult (select (Variables|Hidden|GetSliding) (Variables|Hidden|GetFloor%20Hit) (.HitResult (Utilities|Struct|BreakFindFloorResult (Variables|/Script/Engine.CharacterMovementComponent|GetCurrentFloor (Variables|Character|GetCharacterMovement))))))))
        (bind _returnvalue (Class|ISlideable|IsSlideable(Message) (.HitActor (Collision|BreakHitResult (select (Variables|Hidden|GetSliding) (Variables|Hidden|GetFloor%20Hit) (.HitResult (Utilities|Struct|BreakFindFloorResult (Variables|/Script/Engine.CharacterMovementComponent|GetCurrentFloor (Variables|Character|GetCharacterMovement)))))))))
        (bind _output_get (Variables|Hidden|SetSliding _returnvalue))
        (Utilities|PassonChange _output_get false)
        (Pawn|Components|CharacterMovement|SetMovementMode _charactermovement (select (Variables|Hidden|GetSliding) "MOVE_Flying" "MOVE_Walking") 0)
        (Variables|/Script/Engine.CharacterMovementComponent|SetMaxAcceleration _charactermovement (select (Variables|Hidden|GetSliding) (* (Components|Movement|GetGravityZ (Variables|Character|GetCharacterMovement)) -1.0) (Variables|Hidden|GetMax%20Acceleration)))))
    (:then_1
      (Transformation|SetActorLocation (* (Transformation|GetActorLocation) "1.000000,0.000000,1.000000") false false)
      (if (Variables|Hidden|GetInChill)
        (Variables|Default|SetAlowedTimeInChill (- (Variables|Default|GetAlowedTimeInChill) DeltaSeconds))))
    (:then_2
      (if (or (< (Variables|Default|GetAlowedTimeInChill) 0.0) (< (.z (Transformation|GetActorLocation)) (Variables|Default|GetKillZ)))
        (CallFunction|Reset)))))

(event Input|ActionEvents|InputActionJump
  (params (Key :type Key%20Structure :default "None"))
  ;[0.05104 0.05104 0.05104] Movement
  (:Pressed
    (Character|Jump))
  (:Released
    (Character|StopJumping)))

(event Input|AxisEvents|InputAxisMove
  (params (AxisValue :type Float%20%28single-precision%29))
  (bind _returnvalue (Transformation|GetActorLocation))
  (bind _capsulecomponent (Variables|Collision|GetCapsuleComponent))
  (bind _charactermovement (Variables|Character|GetCharacterMovement))
  (bind _charactermovement_2 (Variables|Character|GetCharacterMovement))
  (bind _returnvalue_2 (Components|Movement|GetGravityZ _charactermovement))
  (bind _returnvalue_3 (Class|CharacterMovementComponent|GetMaxAcceleration _charactermovement))
  (bind _capsuleradius (Variables|/Script/Engine.CapsuleComponent|GetCapsuleRadius _capsulecomponent))
  (bind _capsulehalfheight (Variables|/Script/Engine.CapsuleComponent|GetCapsuleHalfHeight _capsulecomponent))
  (bind _returnvalue_4 (- _capsulehalfheight _capsuleradius))
  (bind _returnvalue_5 (/ _returnvalue_2 _returnvalue_3))
  (bind _returnvalue_6 (- _returnvalue (Math|Vector|MakeVector 0.0 0.0 _returnvalue_4)))
  ;[0.05104 0.05104 0.05104] Movement
  (if (Utilities|Enum|Equal(Enum) (Variables|/Script/Engine.CharacterMovementComponent|GetMovementMode (Variables|Character|GetCharacterMovement)) "MOVE_Flying")
    ;;[0.2302 0.2302 0.2302] Slide
    ;;;[1 1 1] Update Floor Hit
    (bind (_outhit _returnvalue_7) (Collision|SphereTraceByChannel _returnvalue_6 (- _returnvalue_6 (Math|Vector|MakeVector 0.0 0.0 2.0)) (+ (Components|Capsule|GetScaledCapsuleRadius (Variables|Collision|GetCapsuleComponent)) 5.0) "TraceTypeQuery1" false 0 "None"))
    (Variables|Hidden|SetFloor%20Hit _outhit)
    (if _returnvalue_7
      (Class|PawnMovementComponent|AddInputVector _charactermovement_2 (+ (Math|Vector|MakeVector (- (.X (Math|Vector|BreakVector (* (* (Math|Vector|MakeVector (.Z (Math|Vector|BreakVector (.ImpactNormal (Collision|BreakHitResult (Variables|Hidden|GetFloor%20Hit))))) 0.0 (.X (Math|Vector|BreakVector (.ImpactNormal (Collision|BreakHitResult (Variables|Hidden|GetFloor%20Hit)))))) "1.000000,0.000000,-1.000000") AxisValue))) (* (Math|Float|Min(Float) (Math|Vector|DotProduct (* (* (Math|Vector|MakeVector (.Z (Math|Vector|BreakVector (.ImpactNormal (Collision|BreakHitResult (Variables|Hidden|GetFloor%20Hit))))) 0.0 (.X (Math|Vector|BreakVector (.ImpactNormal (Collision|BreakHitResult (Variables|Hidden|GetFloor%20Hit)))))) "1.000000,0.000000,-1.000000") AxisValue) "0.000000,0.000000,1.000000") (Math|Float|Absolute(Float) (.X (Math|Vector|BreakVector (* (* (Math|Vector|MakeVector (.Z (Math|Vector|BreakVector (.ImpactNormal (Collision|BreakHitResult (Variables|Hidden|GetFloor%20Hit))))) 0.0 (.X (Math|Vector|BreakVector (.ImpactNormal (Collision|BreakHitResult (Variables|Hidden|GetFloor%20Hit)))))) "1.000000,0.000000,-1.000000") AxisValue))))) (Math|Float|Sign(Float) (.X (Math|Vector|BreakVector (* (* (Math|Vector|MakeVector (.Z (Math|Vector|BreakVector (.ImpactNormal (Collision|BreakHitResult (Variables|Hidden|GetFloor%20Hit))))) 0.0 (.X (Math|Vector|BreakVector (.ImpactNormal (Collision|BreakHitResult (Variables|Hidden|GetFloor%20Hit)))))) "1.000000,0.000000,-1.000000") AxisValue)))) (Variables|Default|GetHillSlideFactor))) 0.0 (* (Math|Float|Absolute(Float) (.Z (Math|Vector|BreakVector (* (* (Math|Vector|MakeVector (.Z (Math|Vector|BreakVector (.ImpactNormal (Collision|BreakHitResult (Variables|Hidden|GetFloor%20Hit))))) 0.0 (.X (Math|Vector|BreakVector (.ImpactNormal (Collision|BreakHitResult (Variables|Hidden|GetFloor%20Hit)))))) "1.000000,0.000000,-1.000000") AxisValue)))) -1.0)) (Math|Vector|MakeVector 0.0 0.0 _returnvalue_5)) false)
      (else
        (Class|PawnMovementComponent|AddInputVector _charactermovement_2 (Math|Vector|MakeVector (* (Variables|/Script/Engine.CharacterMovementComponent|GetAirControl _charactermovement_2) AxisValue) 0.0 _returnvalue_5) false)))
    (else
      (Class|PawnMovementComponent|AddInputVector (Variables|Character|GetCharacterMovement) (Math|Vector|MakeVector (select (== AxisValue 0.0) (* (Math|Float|Sign(Float) (.x (Variables|/Script/Engine.MovementComponent|GetVelocity (Variables|Character|GetCharacterMovement)))) -1.0) AxisValue) 0.0 0.0) false))))

(fn ConstructionScript
  (Transformation|SetActorLocation (* (Transformation|GetActorLocation) "1.000000,0.000000,1.000000") false false))