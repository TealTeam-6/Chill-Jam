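; BP_ChillSphere is a growing chill area that springs toward the cursor's hit point on Destructible objects and leaves a trail.
; The construction script flattens it to Y=0 and adds overlap meshes, which a timed loop cycles so each tick moves one to the current location and radius.
; Tick diffs overlapping actors against ChilledActors, sending apply or unapply chill messages.
; The chill character's OnReset restores starting position and radius.
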(event Custom|Reset
  (Variables|Default|SetRadius (Utilities|GetClassDefaults "BP_ChillSphere_C"))
  (Transformation|SetActorLocation (Variables|Default|GetInitalLocation) false false)
  (Transformation|SetWorldTransform (Variables|Default|GetOverlapMeshes) (Math|Transform|MakeTransform (Variables|Default|GetInitalLocation) "0, 0, 0" (Math|Vector|MakeVector (Variables|Default|GetRadius) 1.0 (Variables|Default|GetRadius))) false false))

(event EventTick
  (params (DeltaSeconds :type Float%20%28single-precision%29))
  (bind _overlappingactors (Collision|GetOverlappingActors 0 :!class /Script/Engine.Actor))
  (Variables|Default|SetRadius (+ (Variables|Default|GetRadius) (* DeltaSeconds (Variables|Default|GetRadiusGrowth))))
  (bind _returnvalue (Class|KismetMathLibrary|VectorSpringInterp (Transformation|GetActorLocation) (.Location (Collision|BreakHitResult (.HitResult (Class|PlayerController|GetHitResultUnderCursorforObjects (Game|GetPlayerController 0) (Utilities|Array|MakeArray "ObjectTypeQuery6") true)))) (Variables|Default|GetSpring%20State) 1e+02 0.2 DeltaSeconds 1e+01 1.0))
  (Utilities|FlowControl|Sequence
    (:then_0
      (Transformation|SetWorldTransform (Utilities|Array|Get(acopy) (Variables|Default|GetOverlapMeshes) (Variables|Default|GetSelectedSpline)) (Math|Transform|MakeTransform (Transformation|GetActorLocation) "0, 0, 0" (Math|Vector|MakeVector (Variables|Default|GetRadius) 1.0 (Variables|Default|GetRadius))) false false)
      ;[1 1 1] Update Chilled
      (bind _result (Utilities|Set|ToArray (Variables|Default|GetChilledActors)))
      (for _array_element _result
        (if (not (Utilities|Array|ContainsItem _overlappingactors _array_element))
          (Class|IChillable|UnappllyChill(Message) _array_element)
          (Utilities|Set|Remove (Variables|Default|GetChilledActors) _array_element)))
      (for _array_element_2 _overlappingactors
        (if (not (Utilities|Set|Contains (Variables|Default|GetChilledActors) _array_element_2))
          (Class|IChillable|ApplyChill(Message) _array_element_2)
          (Utilities|Set|Add (Variables|Default|GetChilledActors) _array_element_2))))
    (:then_1
      (Transformation|SetActorLocation _returnvalue false false))))

(event EventBeginPlay
  (Variables|Default|SetInitalLocation (Transformation|GetActorLocation))
  (EventDispatchers|BindEventtoOnReset (CallFunction|GetChillCharacter) (delegate Custom|Reset))
  (Utilities|FlowControl|Delay (/ (Variables|Default|GetTail%20Length) (Variables|Default|GetResolution)) :!label _label)
  (Variables|Default|SetSelectedSpline (Math|Integer|%(Integer) (+ (Variables|Default|GetSelectedSpline) 1) (Variables|Default|GetResolution)))
  (goto _label))

(fn ConstructionScript
  (Transformation|SetActorLocation (* (Transformation|GetActorLocation) "1.000000,0.000000,1.000000") false false)
  (for _index (range 1 (Variables|Default|GetResolution))
    (bind _returnvalue (AddComponent|AddStaticMeshComponent false))
    (Utilities|Array|Add (Variables|Default|GetOverlapMeshes) _returnvalue)))